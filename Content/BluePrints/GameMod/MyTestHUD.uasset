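; MyTestHUD manages switching between the player UI widget and the inventory (backpack) widget.
; On BeginPlay it enables input on itself for player 0 and shows the player UI.
; The BackPackOpen/Close action drives a FlipFlop that alternates between the two screens.
; Each switch removes the current widget from its parent, clears its reference, and creates the other widget fresh in the viewport.
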(event EventBeginPlay
  (Utilities|FlowControl|Sequence
    (:then_0
      (Input|EnableInput (Game|GetPlayerController 0)))
    (:then_1
      (CallFunction|CreatPlayerUI))))

(event Input|ActionEvents|InputActionBackPackOpen/Close
  (params (Key :type Key%20Structure :default "None"))
  (:Pressed
    (Utilities|FlowControl|FlipFlop
      (:A
        (Utilities|FlowControl|Sequence
          (:then_0
            (CallFunction|RemovePlayerUI))
          (:then_1
            (CallFunction|CreatInventoryUI))))
      (:B
        (Utilities|FlowControl|Sequence
          (:then_0
            (CallFunction|RemoveInventoryUI))
          (:then_1
            (CallFunction|CreatPlayerUI)))))))

(fn ConstructionScript)

(fn CreatPlayerUI
  ;[1 1 1] 创建角色UI
  (bind _returnvalue (UserInterface|CreateWidget "/Game/UI/MyTestUI.MyTestUI_C" (Game|GetPlayerController 0)))
  (bind _output_get (Variables|Default|SetPlayerUI _returnvalue))
  (UserInterface|Viewport|AddtoViewport _output_get 0) ; 添加到屏幕上
)

(fn RemovePlayerUI
  (Utilities|IsValid (Variables|Default|GetPlayerUI)
    (:Is%20Valid
      (Widget|RemovefromParent (Variables|Default|GetPlayerUI))
      (Variables|Default|SetPlayerUI 0))))

(fn CreatInventoryUI
  ;[1 1 1] 创建角色UI
  (bind _returnvalue (UserInterface|CreateWidget "/Game/UI/MyTestInventoryUI.MyTestInventoryUI_C" (Game|GetPlayerController 0)))
  (bind _output_get (Variables|Default|SetBackPackUI _returnvalue))
  (UserInterface|Viewport|AddtoViewport _output_get 0) ; 添加到屏幕上
)

(fn RemoveInventoryUI
  (Utilities|IsValid (Variables|Default|GetBackPackUI)
    (:Is%20Valid
      (Widget|RemovefromParent (Variables|Default|GetBackPackUI))
      (Variables|Default|SetBackPackUI 0))))