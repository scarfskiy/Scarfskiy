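; Wave-survival game mode that spawns monsters at random TargetPoints, fades in the camera and adds the UI on start.
; A looping timer spawns each wave, whose size grows with wave number and difficulty.
; EndWave re-calls itself after a delay and also fires when registered enemies are cleared.
; Win prints once the wave count reaches the base spawn count; player death stops spawning.
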(event Custom|PlayerDead
  (Variables|Game|SetIsPlayerDead true)
  (Utilities|Time|ClearTimerbyFunctionName 0 "SpawnSingleEnemy"))

(event Custom|EndWave
  (if (not (Variables|Game|GetIsPlayerDead))
    (Utilities|FlowControl|Sequence
      (:then_0
        (CallFunction|SetNextWaveRemainSpawnNum))
      (:then_1
        (Utilities|FlowControl|Delay (Variables|SpawnEnemy|GetWaveFrequency))
        (if (<= (- (Variables|SpawnEnemy|GetBaseSpawnEnmeyNum) (Variables|SpawnEnemy|GetCurrentWave)) 0)
          (Development|PrintString "WIN!!!")
          (else
            (SpawnEnemy|SpawnWave)
            (CallFunction|EndWave)))))))

(event EventBeginPlay
  (Utilities|FlowControl|Sequence
    (:then_0
      (CameraFades|StartCameraFade :self (Game|GetPlayerCameraManager 0) :FromAlpha 1.0 :ToAlpha 0.0 :Duration 2.0 :bHoldWhenFinished true)
      (Utilities|FlowControl|Delay 2.0))
    (:then_1
      ;[1 1 1] 创建角色UI
      (bind _returnvalue (UserInterface|CreateWidget "/Game/UI/MyTestUI.MyTestUI_C" (Game|GetPlayerController 0)))
      (UserInterface|Viewport|AddtoViewport _returnvalue 0) ; 添加到屏幕上
    )
    (:then_2
      (Variables|SpawnEnemy|SetEnemyRemainSpawnNum (Variables|SpawnEnemy|GetBaseSpawnEnmeyNum)) ; 在游戏开始时，将设定的怪物生成数量赋予给波次内怪物生成剩余数变量
    )
    (:then_3
      (SpawnEnemy|GetAllSpawnPoint))
    (:then_4
      (SpawnEnemy|SpawnWave)
      (CallFunction|EndWave))
    (:then_5
      (EventDispatchers|BindEventtoPlayerDead (.AsMy%20Test%20Player (Utilities|Casting|CastToMyTestPlayer (Game|GetPlayerCharacter 0))) (delegate Custom|PlayerDead)))))

(fn ConstructionScript)

(fn GetAllSpawnPoint
  (bind _outactors (Actor|GetAllActorsOfClass "/Script/Engine.TargetPoint"))
  (Variables|Default|SetAllSpawnPointsRef _outactors))

(fn GetRandowSpawnPoint
  (bind _allspawnpointsref (Variables|Default|GetAllSpawnPointsRef))
  (return (Utilities|Array|Get(acopy) _allspawnpointsref (Math|Random|RandomIntegerinRange 0 (Utilities|Array|LastIndex _allspawnpointsref)))))

(fn SpawnWave
  (Math|Integer|IncrementInt (Variables|SpawnEnemy|GetCurrentWave) ; ++波次
    (:%20%20
      (Utilities|Time|SetTimerbyFunctionName 0 "SpawnSingleEnemy" (Variables|SpawnEnemy|GetSpawnFrequency) true) ; 在一个波次中 每隔一个间隔生成一个Actor（调用函数
    )))

(fn SpawnSingleEnemy
  (bind _spawnpoint (SpawnEnemy|GetRandowSpawnPoint))
  (Utilities|IsValid _spawnpoint
    (:Is%20Valid
      (bind _returnvalue (Game|SpawnActorfromClass "/Game/BluePrints/BP/Monster/BP_MyTestMonster.BP_MyTestMonster_C" (Transformation|GetActorTransform _spawnpoint) "Undefined" 0 0)) ; 生成一个Actor
      (Development|PrintString "Spawn a Enemy" true true "(R=0.000000,G=1.000000,B=0.105171,A=1.000000)" 1e+01)
      (Utilities|IsValid _returnvalue ; 防止在出生的一瞬间被秒杀导致的报错
        (:Is%20Valid
          (Utilities|Array|Add (Variables|Default|GetAllEnemyRefs) _returnvalue) ; 将生成的数据添加到AllEnemyRefs数组中进行登记
          (bind _result (Math|Integer|DecrementInt (Variables|SpawnEnemy|GetEnemyRemainSpawnNum)) ; 记录剩余生成数量
            (:%20%20
              (if (== _result 0) ; 判断计数是否归零
                ;[1 1 1] 在波次生成的函数中进行了按时间生成
                (Utilities|Time|ClearTimerbyFunctionName 0 "SpawnSingleEnemy") ; 在生成完成后,清除按事件循环生成Actor的事件
              ))))))))

(fn RegisterEnemyDeath
  (params (Item :type BP%20My%20Test%20Monster%20Object%20Reference%20%28by%20ref%29))
  (Utilities|Array|RemoveItem (Variables|Default|GetAllEnemyRefs) Item)
  (if (SpawnEnemy|IsCurentWaveComplete)
    (CallFunction|EndWave)))

(fn IsCurentWaveComplete
  (return (and (== (Utilities|Array|Length (Variables|Default|GetAllEnemyRefs)) 0) (== (Variables|SpawnEnemy|GetEnemyRemainSpawnNum) 0))))

(fn SetNextWaveRemainSpawnNum
  (Variables|SpawnEnemy|SetEnemyRemainSpawnNum (+ (Variables|SpawnEnemy|GetBaseSpawnEnmeyNum) (Math|Float|Round (* (Variables|SpawnEnemy|GetCurrentWave) (Variables|SpawnEnemy|GetDegreeDifficulty))))))