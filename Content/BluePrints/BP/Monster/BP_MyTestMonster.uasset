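; Test melee monster that chases the player and attacks with a random montage section when in range.
; BeginPlay links the health bar widget, spawns a controller and loops AIMoveTo; Tick starts attacks, pausing movement until they finish.
; DamagePlayer rechecks distance against a scaled range, so players can escape hits.
; At zero HP it may drop an HP pickup, launches its physics capsule along the player's gun direction, then scales the mesh and destroys itself.
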(event Custom|PlayerDeadEvent
  (Variables|Monster|SetIsPlayerDead true)
  (ActiveMovment|DeactiveAiMovment))

(event EventBeginPlay
  (Utilities|FlowControl|Sequence
    (:then_0
      ;[1 1 1] 挂载血条,给血条传递数据
      (Variables|/Game/UI/EnemyUI_01.EnemyUI_01_C|SetEnemy (.AsEnemy%20UI%2001 (Utilities|Casting|CastToEnemyUI_01 (UserInterface|GetUserWidgetObject (Variables|组件|GetWidget)))) self))
    (:then_1
      (Pawn|SpawnDefaultController) ; 给Actor生成控制器,否则不会寻路
      ;[1 1 1] 在Spawn时,不会生成这种简单AI的AI控制器,因此寻路会失效
      (AI|AIMoveTo self "0, 0, 0" (Game|GetPlayerCharacter 0) 1.0 false :!label _label
        (:OnSuccess
          _)
        (:OnFail
          _))
      (Utilities|FlowControl|Delay 0.5)
      (Utilities|IsDeadMacro
        (:false
          (goto _label))))
    (:then_2
      (EventDispatchers|AssignPlayerDead (.AsMy%20Test%20Player (Utilities|Casting|CastToMyTestPlayer (Game|GetPlayerCharacter 0))) (delegate Custom|PlayerDeadEvent)))))

(event EventTick
  (params (DeltaSeconds :type Float%20%28single-precision%29))
  (if (Attack|CanAttack)
    (Utilities|FlowControl|Sequence
      (:then_0
        (ActiveMovment|DeactiveAiMovment))
      (:then_1
        (Animation|Montage|PlayMontage (Variables|Character|GetMesh) "/Game/Animations/Monster/AM_TestMonster_Attack.AM_TestMonster_Attack" 1.0 0.0 (Attack|GetRandonAttackMontageSectionName)
          (:OnCompleted
            (Utilities|IsDeadMacro
              (:false
                (ActiveMovment|ActiveAiMovment) ; 播放完成后激活
              ))))))))

(event Game|Damage|EventAnyDamage
  (params (Damage :type Float%20%28single-precision%29) (DamageType :type Damage%20Type%20Object%20Reference) (InstigatedBy :type Controller%20Object%20Reference) (DamageCauser :type Actor%20Object%20Reference))
  ;[1 0 0] 受击
  (bind _hp (EnemyProperty|ReduceHP Damage))
  (if (<= _hp 0.0)
    (Variables|Monster|SetIsDead true)
    (Utilities|FlowControl|DoOnce false
      (:Completed
        (Utilities|FlowControl|Sequence
          (:then_0
            (ActiveMovment|DeactiveAiMovment))
          (:then_1
            (CallFunction|SpawnHpTool))
          (:then_2
            ;;[1 1 1] 布娃娃
            (CallFunction|SetRagdollEffect))
          (:then_3
            (Utilities|FlowControl|Delay 3.0)
            (bind _scale (Timeline|ScaleLine Play)
              (:Update
                (Transformation|SetWorldScale3D (Variables|Character|GetMesh) (Math|Conversions|ToVector(Float) _scale))
                (Utilities|FlowControl|Delay (Components|Timeline|GetTimelineLength (Variables|Default|GetScaleLine)))
                (Actor|DestroyActor) ; 死完自己销毁
              ))))))))

(fn ConstructionScript)

(fn DamagePlayer
  (if (Attack|IsPlayerEscapeinAttackRange) ; 玩家是否在攻击范围内
    (Game|Damage|ApplyDamage (Game|GetPlayerCharacter 0) (Variables|Attack|GetDamagePerHit) 0 0)))

(fn IsPlayerinAttackRange
  (return (<= (Transformation|GetDistanceTo (Game|GetPlayerCharacter 0)) (Variables|Attack|GetAttackRange))))

(fn IsAttacking
  (return (Animation|Montage|MontageIsPlaying (Components|SkeletalMesh|GetAnimInstance (Variables|Character|GetMesh)) "/Game/Animations/Monster/AM_TestMonster_Attack.AM_TestMonster_Attack")) ; 因为攻击于动画蒙太奇有关,因此判断蒙太奇是否在播放就能知晓是否正在攻击
)

(fn CanAttack
  (return (Math|Boolean|ANDBoolean (Attack|IsPlayerinAttackRange) (not (Attack|IsAttacking)) (not (Variables|Monster|GetIsDead)) (not (Variables|Monster|GetIsPlayerDead)))))

(fn GetRandonAttackMontageSectionName
  (return (Utilities|String|StringToName (Utilities|String|ToString(Integer) (Math|Random|RandomIntegerinRange 1 3)))) ; 因为片段使用了数字命名,因此可以用Int转换到name的方式输出随机播放
)

(fn ActiveAiMovment
  (Components|Activation|Activate (Variables|Character|GetCharacterMovement) false) ; 激活设定的目标
)

(fn DeactiveAiMovment
  (bind _charactermovement (Variables|Character|GetCharacterMovement))
  (Utilities|FlowControl|Sequence
    (:then_0
      (Components|Movement|StopMovementImmediately _charactermovement) ; 立即停止设定目标的运动
    )
    (:then_1
      (Components|Activation|Deactivate _charactermovement) ; 停止激活设定的目标
    )))

(fn IsPlayerEscapeinAttackRange
  (return (<= (Transformation|GetDistanceTo (Game|GetPlayerCharacter 0)) (* (Variables|Attack|GetAttackRange) (Variables|Attack|GetAttackRangeFacter)))) ; 当玩家距离怪物超过攻击距离2倍,输出攻击判定失效
)

(fn ReduceHP
  (params (Damege :type Float%20%28single-precision%29))
  (bind _output_get (Variables|Monster|SetHP (Math|Float|Clamp(Float) (- (Variables|Monster|GetHP) Damege) 0.0 (Variables|Monster|GetMaxHP))))
  (return _output_get))

(fn SetRagdollEffect
  (bind _returnvalue (Game|GetPlayerCharacter 0))
  (bind _returnvalue_2 (Math|Random|RandomFloatinRange 1e+02 3e+02))
  (bind _capsulecomponent (Variables|Collision|GetCapsuleComponent))
  (bind _asmy_test_player (Utilities|Casting|CastToMyTestPlayer _returnvalue))
  (bind _sk_gun (Variables|/Game/BluePrints/BP/player/MyTestPlayer.MyTestPlayer_C|GetSK_Gun _asmy_test_player))
  (bind _returnvalue_3 (Transformation|GetSocketRotation _sk_gun "None"))
  (bind _returnvalue_4 (Math|Vector|GetForwardVector _returnvalue_3))
  (Utilities|FlowControl|Sequence
    (:then_0
      (Physics|SetSimulatePhysics _capsulecomponent true) ; 启用模拟物理
    )
    (:then_1
      (Physics|AddImpulse _capsulecomponent (Math|Vector|MakeVector (* (.x _returnvalue_4) _returnvalue_2) (* (.y _returnvalue_4) _returnvalue_2) _returnvalue_2) "None" true))))

(fn SpawnHpTool
  (if (<= (Math|Random|RandomFloat) (Variables|Default|GetSpawnFactor))
    (Game|SpawnActorfromClass "/Game/BluePrints/BP/PickUps/BP_HpTool.BP_HpTool_C" (Transformation|GetActorTransform) "Undefined" 0 0) ; 生成类
  ))