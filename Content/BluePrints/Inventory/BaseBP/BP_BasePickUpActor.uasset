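; Base pickup actor for inventory items that notifies the player when they come near or move away.
; On BeginPlay it writes itself into its ItemInfo struct as the scene instance reference, applies the item mass to its static mesh and prints a debug string.
; Sphere overlap begin and end cast to MyTestPlayer and pass ItemInfo to its functions that show or clear the nearby-item display.
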(event EventBeginPlay
  (bind _output_get (Variables|Default|SetItemInfo (Utilities|Struct|MakePickUpItem (.name (Variables|Default|GetItemInfo)) (.itemtype (Variables|Default|GetItemInfo)) (.mass (Variables|Default|GetItemInfo)) (.itemclass (Variables|Default|GetItemInfo)) self (.icon (Variables|Default|GetItemInfo)))))
  (Class|PrimitiveComponent|SetMassOverrideinKg (Variables|Default|GetStaticMesh) "None" (.mass _output_get) true)
  (Development|PrintString "Hello"))

(event OnComponentBeginOverlap(Sphere)
  (params (OverlappedComponent :type Primitive%20Component%20Object%20Reference) (OtherActor :type Actor%20Object%20Reference) (OtherComp :type Primitive%20Component%20Object%20Reference) (OtherBodyIndex :type Integer) (bFromSweep :type Boolean) (SweepResult :type Hit%20Result%20Structure%20%28by%20ref%29))
  ;[1 1 1] 将碰撞设置为只对pawn起效
  (bind _asmy_test_player (Utilities|Casting|CastToMyTestPlayer OtherActor))
  (Default|接近物体显示 _asmy_test_player (Variables|Default|GetItemInfo)))

(event OnComponentEndOverlap(Sphere)
  (params (OverlappedComponent :type Primitive%20Component%20Object%20Reference) (OtherActor :type Actor%20Object%20Reference) (OtherComp :type Primitive%20Component%20Object%20Reference) (OtherBodyIndex :type Integer))
  ;[1 1 1] 将碰撞设置为只对pawn起效
  (bind _asmy_test_player (Utilities|Casting|CastToMyTestPlayer OtherActor))
  (Default|远离物体清除显示 _asmy_test_player (Variables|Default|GetItemInfo)))

(fn ConstructionScript
  ;[1 1 1] 初始化数据
)